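; Airship fleet manager actor that tracks built and destroyed airships and dispatches them on routes.
; SendFirstOnRoute gives a route to the first available airship and reports whether one was found, while getters count total and available ships.
; One second after BeginPlay, a one-shot timer gathers every EmptyWaypoint in the level into a route and dispatches it.
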(event Custom|Send
  (bind _newvar_0 (Variables|Default|GetNewVar_0))
  (bind _outactors (Actor|GetAllActorsOfClass "/Game/Blueprints/EmptyWaypoint.EmptyWaypoint_C"))
  (for _array_element _outactors
    (Utilities|Array|AddUnique _newvar_0 _array_element))
  (CallFunction|SendFirstonRoute (Utilities|Struct|MakeRouteStruct _newvar_0 "0.000000,0.000000,0.000000" 0 true)))

(event EventBeginPlay
  (Utilities|Time|SetTimerbyEvent (delegate Custom|Send) 1.0))

(event Collision|EventActorBeginOverlap
  (params (OtherActor :type Actor%20Object%20Reference)))

(event EventTick
  (params (DeltaSeconds :type Float%20%28single-precision%29)))

(fn ConstructionScript)

(fn AirshipBuilt
  (params (Airship :type Airship%20Object%20Reference))
  (Utilities|Array|AddUnique (Variables|Default|GetAirships) Airship))

(fn AirshipDestroyed
  (params (Airship :type Airship%20Object%20Reference))
  (Utilities|Array|RemoveItem (Variables|Default|GetAirships) Airship))

(fn SendFirstonRoute
  (params (Route :type Route%20Struct%20Structure))
  (bind _array_element (Utilities|Array|ForEachLoopwithBreak (Variables|Default|GetAirships) :!label _label)
    (:LoopBody
      (if (Default|IsAvailable _array_element)
        (Default|AssignRoute _array_element Route)
        (LocalVariables|SetFound true)
        (goto _label Break)))
    (:Completed
      (return (LocalVariables|GetFound)))))

(fn GetTotalShips
  (return (Utilities|Array|Length (Variables|Default|GetAirships))))

(fn GetAvailableShips
  (bind _counter (LocalVariables|Getcounter))
  (for _array_element (Variables|Default|GetAirships)
    (if (Default|IsAvailable _array_element)
      (Math|Integer|IncrementInt _counter)))
  (return _counter))