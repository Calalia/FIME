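; FIMEGameInstance is a game instance Blueprint that stores the game's shared economy state: houses, ships and a resource struct.
; Getters expose that state, while GetWorkerAmounts is an empty stub.
; AddResources merges amounts into the stored struct through a helper and always returns true.
; UseResources commits a subtraction only when the helper reports success, returning false otherwise.
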(fn GetHouses
  (return (Variables|Default|GetHouses)))

(fn GetShips
  (return (Variables|Default|GetShips)))

(fn GetResourceStruct
  (return (Variables|Default|GetResourceStruct)))

(fn GetWorkerAmounts)

(fn AddResources
  (params (ResourcesToAdd :type Resource%20Struct%20Structure))
  (Variables|Default|SetResourceStruct (.Added (CallFunction|AddResources ResourcesToAdd (Variables|Default|GetResourceStruct))))
  (return true))

(fn UseResources
  (params (ResourcesToUse :type Resource%20Struct%20Structure))
  (if (.Success (CallFunction|SubtractResources (Variables|Default|GetResourceStruct) ResourcesToUse))
    (Variables|Default|SetResourceStruct (.Subtracted (CallFunction|SubtractResources (Variables|Default|GetResourceStruct) ResourcesToUse)))
    (return true)
    (else
      (return false))))