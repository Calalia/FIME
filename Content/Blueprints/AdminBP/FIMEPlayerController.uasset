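; Player controller for a top-down building game that drives the camera pawn and handles mouse selection and building placement.
; Axis input, screen-edge scrolling and gated pan move the camera, with speed scaled by zoom distance.
; Left click places the ghost building, selects Selectables or opens a build menu on build-area hits; in build mode the zoom axis rotates the ghost.
; It also creates the HUD and has a test key toggling timed resource income.
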(event Custom|AddResources
  ;[1 1 1] E (for testing only)
  (Default|AddResources (Variables|References|GetGameInstanceRef) (Utilities|Struct|MakeResourceStruct 4 2 3 1)))

(event EventBeginPlay
  ;[1 1 1] BeginPlay
  (Variables|Default|SetbShowMouseCursor true)
  (|CreateReferences)
  (bind _returnvalue (UserInterface|CreateWidget "/Game/Blueprints/Widgets/OnScreenUI.OnScreenUI_C" self (Variables|References|GetGameInstanceRef)))
  (UserInterface|Viewport|AddtoViewport _returnvalue 0))

(event Input|ActionEvents|InputActionPan
  (params (Key :type Key%20Structure))
  (bind _camerapawnref (Variables|References|GetCameraPawnRef))
  (bind _returnvalue (Transformation|GetActorRotation _camerapawnref))
  ;[1 1 1] Pan X
  (:Pressed
    (Utilities|FlowControl|Gate true) ; enters at Open
  )
  (:Released
    (Utilities|FlowControl|Gate true) ; enters at Close
  ))

(event Input|ActionEvents|InputActionPan
  (params (Key :type Key%20Structure))
  (bind _camerapawnref (Variables|References|GetCameraPawnRef))
  (bind _returnvalue (Transformation|GetActorRotation _camerapawnref))
  ;[1 1 1] Pan Y
  (:Pressed
    (Utilities|FlowControl|Gate true) ; enters at Open
  )
  (:Released
    (Utilities|FlowControl|Gate true) ; enters at Close
  ))

(event Input|AxisEvents|InputAxisHorizontal
  (params (AxisValue :type Float%20%28single-precision%29))
  (bind _camerapawnref (Variables|References|GetCameraPawnRef))
  ;[1 1 1] Movement Horizontal
  (if (not (Variables|Default|GetDisableCamMovement))
    (Transformation|SetActorTransform _camerapawnref (Utilities|MovementHorizontal AxisValue (CallFunction|ZoomMovementSpeed) _camerapawnref))))

(event Input|AxisEvents|InputAxisVertical
  (params (AxisValue :type Float%20%28single-precision%29))
  (bind _camerapawnref (Variables|References|GetCameraPawnRef))
  ;[1 1 1] Movement Vertical
  (if (not (Variables|Default|GetDisableCamMovement))
    (Transformation|SetActorTransform _camerapawnref (Utilities|MovementVertical AxisValue (CallFunction|ZoomMovementSpeed) _camerapawnref))))

(event Input|AxisEvents|InputAxisZoom
  (params (AxisValue :type Float%20%28single-precision%29))
  (bind _returnvalue (Game|GetPlayerController 0))
  (bind _ghostbuildingref (Variables|References|GetGhostBuildingRef))
  (bind _camerapawnref (Variables|References|GetCameraPawnRef))
  (bind _returnvalue_2 (Transformation|GetActorTransform _ghostbuildingref))
  (bind (_worldlocation _worlddirection) (Game|Player|ConvertMouseLocationToWorldSpace _returnvalue))
  (bind _springarm (Variables|/Game/Blueprints/CameraPawn.CameraPawn_C|GetSpringArm _camerapawnref))
  ;[1 1 1] Zoom
  (if (Variables|Default|GetBuildModeActive)
    ;[1 1 1] Update GhostBuilding Location if Buildmode Active
    (bind (_outhit _returnvalue_3) (Collision|LineTraceByChannel _worldlocation (+ _worldlocation (* _worlddirection 2e+04)) "TraceTypeQuery3" false 0 "None"))
    (Default|UpdateLocation (Variables|References|GetGhostBuildingRef) (Math|Transform|MakeTransform (select _returnvalue_3 (.location _outhit) (.location _returnvalue_2)) (Math|Rotator|MakeRotator (.roll (.rotation _returnvalue_2)) (.pitch (.rotation _returnvalue_2)) (+ (.yaw (.rotation _returnvalue_2)) AxisValue)) (.scale _returnvalue_2)))
    (else
      (Variables|/Script/Engine.SpringArmComponent|SetTargetArmLength _springarm (Math|Float|Clamp(Float) (+ (Variables|/Script/Engine.SpringArmComponent|GetTargetArmLength _springarm) (* AxisValue (Variables|Default|GetZoomSensitivity))) (Variables|Default|GetMinZoomDistance) (Variables|Default|GetMaxZoomDistance))))))

(event Input|MouseEvents|MouseX
  (params (AxisValue :type Float%20%28single-precision%29))
  (bind _camerapawnref (Variables|References|GetCameraPawnRef))
  (bind _returnvalue (Transformation|GetActorRotation _camerapawnref))
  ;[1 1 1] Pan X
  (Utilities|FlowControl|Sequence
    (:then_0
      (Utilities|FlowControl|Gate true
        (:Exit
          (Transformation|SetActorRotation (Variables|References|GetCameraPawnRef) (Math|Rotator|MakeRotator (.roll _returnvalue) (.pitch _returnvalue) (+ (.yaw _returnvalue) (* (Variables|Default|GetPanSensitivity) AxisValue)))))))
    (:then_1
      ;[1 1 1] Screen Edge Movement
      (if (not (Variables|Default|GetDisableCamMovement))
        (bind (_cammovehorizontal _cammovevertical) (Utilities|ScreenEdgeMovement)
          (:Exec
            (Transformation|AddActorLocalOffset (Variables|References|GetCameraPawnRef) (Math|Vector|MakeVector _cammovevertical _cammovehorizontal 0.0) false false)))))))

(event Input|MouseEvents|MouseY
  (params (AxisValue :type Float%20%28single-precision%29))
  (bind _camerapawnref (Variables|References|GetCameraPawnRef))
  (bind _returnvalue (Transformation|GetActorRotation _camerapawnref))
  ;[1 1 1] Pan Y
  (Utilities|FlowControl|Sequence
    (:then_0
      (Utilities|FlowControl|Gate true
        (:Exit
          (Transformation|SetActorRotation (Variables|References|GetCameraPawnRef) (Math|Rotator|MakeRotator (.roll _returnvalue) (Math|Float|Clamp(Float) (+ (.pitch _returnvalue) (* (Variables|Default|GetPanSensitivity) AxisValue)) -15.0 35.0) (.yaw _returnvalue))))))
    (:then_1
      ;[1 1 1] Screen Edge Movement
      (if (not (Variables|Default|GetDisableCamMovement))
        (Utilities|ScreenEdgeMovement) ; enters at MouseY
      ))))

(event Input|MouseEvents|LeftMouseButton
  (params (Key :type Key%20Structure))
  (bind _returnvalue (Game|GetPlayerController 0))
  (bind (_locationx _locationy) (Game|Player|GetMousePosition))
  (bind _returnvalue_2 (Game|GetPlayerController 0))
  (bind _self self)
  (bind (_worldlocation _worlddirection) (Game|Player|ConvertMouseLocationToWorldSpace _returnvalue))
  (bind (_worldlocation_2 _worlddirection_2) (Game|Player|ConvertMouseLocationToWorldSpace _returnvalue_2))
  ;[1 1 1] Left Mouse Button
  (:Pressed
    (if (Variables|Default|GetBuildModeActive)
      ;;[1 1 1] Try Construct if Buildmode Active
      (bind _success (Default|Construct (Variables|References|GetGhostBuildingRef)))
      (Variables|Default|SetBuildModeActive (not _success))
      (else
        ;;[1 1 1] Trace for selectables if Buildmode Inactive
        (bind (_outhit _returnvalue_3) (Collision|LineTraceByChannel _worldlocation (+ _worldlocation (* _worlddirection 1e+04)) "TraceTypeQuery4" false 0 "None"))
        (if _returnvalue_3
          (bind _asselectable (Utilities|Casting|CastToSelectable (.hitactor _outhit)))
          (Default|Select _asselectable)
          (else
            ;;[1 1 1] Remove old active Widget if there is one
            (CallFunction|TryRemoveActiveWidget)
            ;;[1 1 1] Trace for BuildArea and create build Widget
            (bind _returnvalue_4 (Collision|LineTraceByChannel _worldlocation_2 (+ _worldlocation_2 (* _worlddirection_2 2e+04)) "TraceTypeQuery3" false 0 "None"))
            (if _returnvalue_4
              (bind _returnvalue_5 (UserInterface|CreateWidget "/Game/Blueprints/Widgets/BuildMenuWidget.BuildMenuWidget_C" _self _self (Variables|References|GetGameInstanceRef)))
              (Class|UserWidget|SetPositioninViewport _returnvalue_5 (Math|Vector2D|MakeVector2D _locationx _locationy) true)
              (UserInterface|Viewport|AddtoViewport _returnvalue_5 0)
              (Variables|Default|SetActiveWidget _returnvalue_5))))))))

(event Input|KeyboardEvents|E
  (params (Key :type Key%20Structure))
  ;[1 1 1] E (for testing only)
  (:Pressed
    (Utilities|FlowControl|FlipFlop
      (:A
        (bind _returnvalue (Utilities|Time|SetTimerbyEvent (delegate Custom|AddResources) 1.0 true)))
      (:B
        (Utilities|Time|ClearandInvalidateTimerbyHandle _returnvalue)))))

(event Input|MouseEvents|RightMouseButton
  (params (Key :type Key%20Structure))
  ;[1 1 1] Right Mouse Button
  (:Pressed
    (Utilities|FlowControl|Sequence
      (:then_0
        ;;[1 1 1] Deactivate BuildMode
        (if (Variables|Default|GetBuildModeActive)
          (Default|DeactivateGhostBuilding (Variables|References|GetGhostBuildingRef))
          (Variables|Default|SetBuildModeActive false)))
      (:then_1
        ;;[1 1 1] Remove active Widget if there is one
        (CallFunction|TryRemoveActiveWidget)))))

(fn ConstructionScript)

(fn ZoomMovementSpeed
  (return (* (Math|Float|Clamp(Float) (/ (Variables|/Script/Engine.SpringArmComponent|GetTargetArmLength (Variables|/Game/Blueprints/CameraPawn.CameraPawn_C|GetSpringArm (Variables|References|GetCameraPawnRef))) 1e+02) 5.0 2e+01) (Variables|Default|GetMoveSensitivity))))

(fn ActivateBuildmode
  (params (Building :type Build%20Struct%20Structure))
  (bind _ghostbuildingref (Variables|References|GetGhostBuildingRef))
  (Variables|Default|SetBuildModeActive true)
  (Default|DeactivateGhostBuilding _ghostbuildingref)
  (Default|ActivateGhostBuilding _ghostbuildingref Building))

(fn TryRemoveActiveWidget
  (bind _activewidget (Variables|Default|GetActiveWidget))
  (if (Utilities|IsValid _activewidget)
    (Widget|RemovefromParent _activewidget)))