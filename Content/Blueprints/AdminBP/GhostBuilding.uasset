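; GhostBuilding is a placement preview actor that shows a building's ghost mesh before construction.
; Activation stores a BuildStruct and sets its mesh, while location updates move the actor and write the transform into that struct.
; While active, Tick colours the mesh red when overlapping ParentBuilding actors, otherwise green.
; Construct spawns the struct's proxy class at that transform without checking overlaps, then deactivates and clears the ghost.
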(event OnComponentBeginOverlap(BuildingMesh)
  (params (OverlappedComponent :type Primitive%20Component%20Object%20Reference) (OtherActor :type Actor%20Object%20Reference) (OtherComp :type Primitive%20Component%20Object%20Reference) (OtherBodyIndex :type Integer) (bFromSweep :type Boolean) (SweepResult :type Hit%20Result%20Structure%20%28by%20ref%29)))

(event Custom|Construct
  (bind _buildstruct (Variables|Default|GetBuildStruct))
  (Game|SpawnActorfromClass (.proxyclass _buildstruct) (.transform _buildstruct) "Undefined" 0 (Variables|Default|GetBuildStruct) 0)
  (CallFunction|DeactivateGhostBuilding))

(event EventTick
  (params (DeltaSeconds :type Float%20%28single-precision%29))
  (bind _buildingmesh (Variables|Default|GetBuildingMesh))
  (if (Variables|Default|GetIsActive)
    (if (> (Utilities|Array|Length (Collision|GetOverlappingActors "/Game/Blueprints/ParentBuilding.ParentBuilding_C" :!class /Script/Engine.Actor)) 0)
      (Rendering|Material|SetMaterial _buildingmesh 0 "/Game/Materials/BasicRed.BasicRed")
      (else
        (Rendering|Material|SetMaterial _buildingmesh 0 "/Game/Materials/BasicGreen.BasicGreen")))))

(fn ConstructionScript)

(fn ActivateGhostBuilding
  (params (BuildStruct :type Build%20Struct%20Structure))
  (bind _output_get (Variables|Default|SetBuildStruct BuildStruct))
  (Components|StaticMesh|SetStaticMesh (Variables|Default|GetBuildingMesh) (.ghostmesh _output_get))
  (Variables|Default|SetIsActive true))

(fn DeactivateGhostBuilding
  (Variables|Default|SetBuildStruct (Utilities|Struct|MakeBuildStruct 0 "/Game/Blueprints/ContructionProxy.ContructionProxy_C" 0))
  (Components|StaticMesh|SetStaticMesh (Variables|Default|GetBuildingMesh) 0)
  (Variables|Default|SetIsActive false))

(fn UpdateLocation
  (params (Location :type Transform))
  (Transformation|SetActorTransform Location)
  (Variables|Default|SetBuildStruct (Utilities|Struct|MakeBuildStruct (.BuildingClass (Utilities|Struct|BreakBuildStruct (Variables|Default|GetBuildStruct))) (.ProxyClass (Utilities|Struct|BreakBuildStruct (Variables|Default|GetBuildStruct))) (.GhostMesh (Utilities|Struct|BreakBuildStruct (Variables|Default|GetBuildStruct))) Location (.BuildTime (Utilities|Struct|BreakBuildStruct (Variables|Default|GetBuildStruct))))))