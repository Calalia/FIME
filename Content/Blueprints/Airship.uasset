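; Airship actor that flies along an assigned route of waypoints and registers its creation and destruction with the game instance's AirshipManager.
; Tick moves it at constant speed toward the current destination, facing travel direction, unless paused, available or eaten.
; On arrival each waypoint's Arrive can pause it; otherwise it advances, looping or becoming available when the route ends.
; NextLocation sets a new destination and resumes movement.
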(event EventBeginPlay
  (|CallParentFunction)
  (if (Utilities|IsValid (Variables|Default|GetGameInstanceRef))
    _
    (else
      (bind _asfimegame_instance (Utilities|Casting|CastToFIMEGameInstance (Game|GetGameInstance)))
      (Variables|Default|SetGameInstanceRef _asfimegame_instance)))
  (bind _output_get (Variables|Default|SetAirshipManagerRef (Variables|/Game/Blueprints/AdminBP/FIMEGameInstance.FIMEGameInstance_C|GetAirshipManager (Variables|Default|GetGameInstanceRef))))
  (Default|AirshipBuilt _output_get self))

(event Collision|EventActorBeginOverlap
  (params (OtherActor :type Actor%20Object%20Reference))
  (|CallParentFunction OtherActor) ; This node is disabled and will not be called.\nDrag off pins to build functionality.
)

(event EventTick
  (params (DeltaSeconds :type Float%20%28single-precision%29))
  (bind _returnvalue (Transformation|GetActorLocation))
  (bind _route (Variables|Default|GetRoute))
  (bind _route_2 (Variables|Default|GetRoute))
  (bind _movementspeed (Variables|AirshipVariables|GetMovementSpeed))
  (bind _returnvalue_2 (- (.currentdestination _route_2) _returnvalue))
  (bind _returnvalue_3 (* DeltaSeconds _movementspeed))
  (bind _returnvalue_4 (Math|Vector|Normalize _returnvalue_2))
  (bind _returnvalue_5 (* _returnvalue_4 _returnvalue_3))
  (|CallParentFunction DeltaSeconds)
  (if (Math|Boolean|ANDBoolean (not (Variables|AirshipVariables|GetPaused)) (not (Variables|AirshipVariables|GetAvailable)) (not (Variables|Default|GetEaten)))
    (if (<= (Math|Vector|VectorLength (- (.currentdestination _route_2) _returnvalue)) (Math|Vector|VectorLength _returnvalue_5))
      ;[1 1 1] Inform waypoint you've arrived and set location
      (Transformation|SetActorLocation (.currentdestination _route) false false)
      (bind _pause (Default|Arrive (Utilities|Array|Get(acopy) (.waypoints _route) (.currentindex _route)) self))
      (Variables|AirshipVariables|SetPaused _pause)
      ;;[1 1 1] Continue if not asked to stop
      (if (not _pause)
        (CallFunction|NextWaypoint))
      (else
        ;[1 1 1] Move towards destination if not there
        (Transformation|SetActorLocation (+ _returnvalue _returnvalue_5) false false)
        (Transformation|SetActorRotation (Math|Rotator|MakeRotfromXZ _returnvalue_4 (Math|Vector|VectorUp)))))))

(event EventDestroyed
  (Default|AirshipDestroyed (Variables|Default|GetAirshipManagerRef) self))

(fn ConstructionScript
  (|CallParentFunction))

(fn IsAvailable
  (return (Variables|AirshipVariables|GetAvailable)))

(fn AssignRoute
  (params (Route :type Route%20Struct%20Structure))
  (if (> (Utilities|Array|Length (.waypoints Route)) 0)
    (bind _location (Default|GetLocation (Utilities|Array|Get(acopy) (.waypoints Route) (.currentindex Route)) self))
    (Variables|Default|SetRoute (Utilities|Struct|MakeRouteStruct (.waypoints Route) _location (.currentindex Route) (.looping Route)))
    (Variables|AirshipVariables|SetPaused false)
    (Variables|AirshipVariables|SetAvailable false)))

(fn NextWaypoint
  (bind _result (Math|Integer|IncrementInt (.currentindex (Variables|Default|GetRoute)))
    (:%20%20
      (if (== _result (Utilities|Array|Length (.waypoints (Variables|Default|GetRoute))))
        (if (.looping (Variables|Default|GetRoute))
          (Variables|Default|SetRoute (Utilities|Struct|MakeRouteStruct (.waypoints (Variables|Default|GetRoute)) (.currentdestination (Variables|Default|GetRoute)) -1 (.looping (Variables|Default|GetRoute))))
          (CallFunction|NextWaypoint)
          (else
            (Variables|AirshipVariables|SetPaused true)
            (Variables|AirshipVariables|SetAvailable true)
            (Variables|Default|SetRoute "")))
        (else
          (bind _location (Default|GetLocation (Utilities|Array|Get(acopy) (.waypoints (Variables|Default|GetRoute)) _result) self))
          (Variables|Default|SetRoute (Utilities|Struct|MakeRouteStruct (.waypoints (Variables|Default|GetRoute)) _location _result (.looping (Variables|Default|GetRoute))))
          (Variables|AirshipVariables|SetPaused false))))))

(fn NextLocation
  (params (Location :type Vector))
  (Variables|Default|SetRoute (Utilities|Struct|MakeRouteStruct (.waypoints (Variables|Default|GetRoute)) Location (.currentindex (Variables|Default|GetRoute)) (.looping (Variables|Default|GetRoute))))
  (Variables|AirshipVariables|SetPaused false))