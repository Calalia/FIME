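; CloudControl is a spawner that fills the level with drifting-cloud actors at random positions below the world origin.
; Each Tick it spawns at most one cloud, topping up large CloudMoveTest2 actors to MaxBigCloudAmount before adding CloudMoveTest ones up to MaxCloudAmount.
; Big clouds use a fixed scale over a wider, lower area, while smaller ones get random per-axis scale.
; Counts come from GetAllActorsOfClass results captured just before the previous spawn.
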(event EventTick
  (params (DeltaSeconds :type Float%20%28single-precision%29))
  (bind _returnvalue (Math|Random|RandomFloatinRange 0.2 1.0))
  (if (< (Utilities|Array|Length (stale _outactors)) (Variables|Default|GetMaxBigCloudAmount))
    (bind _outactors (Actor|GetAllActorsOfClass "/Game/Blueprints/CloudMoveTest2.CloudMoveTest2_C"))
    (Game|SpawnActorfromClass "/Game/Blueprints/CloudMoveTest2.CloudMoveTest2_C" (Math|Transform|MakeTransform (Math|Vector|MakeVector (Math|Random|RandomFloatinRange -1e+05 1e+05) (Math|Random|RandomFloatinRange -6e+05 6e+05) (Math|Random|RandomFloatinRange -7.8e+04 -9.6e+04)) "0, 0, 0" "3.000000,3.000000,3.000000") "Undefined" 0 0)
    (elif (< (Utilities|Array|Length (stale _outactors_2)) (Variables|Default|GetMaxCloudAmount))
      (bind _outactors_2 (Actor|GetAllActorsOfClass "/Game/Blueprints/CloudMoveTest.CloudMoveTest_C"))
      (Game|SpawnActorfromClass "/Game/Blueprints/CloudMoveTest.CloudMoveTest_C" (Math|Transform|MakeTransform (Math|Vector|MakeVector (Math|Random|RandomFloatinRange -1e+05 1e+05) (Math|Random|RandomFloatinRange -3e+05 3e+05) (* _returnvalue -2.2e+04)) "0, 0, 0" (Math|Vector|MakeVector _returnvalue _returnvalue _returnvalue)) "Undefined" 0 0))))

(fn ConstructionScript)