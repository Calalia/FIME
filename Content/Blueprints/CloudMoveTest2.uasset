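; Test cloud mover that drifts a Sphere component along its local Y axis and recycles it, apparently as a looping cloud.
; Each Tick adds Movespeed as a local offset, without delta-time scaling, so drift speed depends on frame rate.
; Once world Y passes CloudMaxDistance, the sphere jumps back to a fixed far-negative Y with random X, height and per-axis scale, so one mesh reappears as differently shaped clouds.
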(event EventTick
  (params (DeltaSeconds :type Float%20%28single-precision%29))
  (bind _returnvalue (Math|Random|RandomFloatinRange 2e+02 8e+02))
  (bind _sphere (Variables|Default|GetSphere))
  (if (> (.y (Transformation|GetWorldLocation _sphere)) (Variables|Default|GetCloudMaxDistance))
    (Transformation|SetWorldTransform _sphere (Math|Transform|MakeTransform (Math|Vector|MakeVector (Math|Random|RandomFloatinRange -1e+05 1e+05) -3e+05 (Math|Random|RandomFloatinRange -7.8e+04 -9.6e+04)) "0, 0, 0" (Math|Vector|MakeVector _returnvalue _returnvalue (/ _returnvalue 1.0))) false false)
    (else
      (Class|SceneComponent|AddLocalTransform _sphere (Math|Transform|MakeTransform (Math|Vector|MakeVector 0.0 (Variables|Default|GetMovespeed) 0.0) "0, 0, 0" "3.000000,3.000000,3.000000") false false))))

(fn ConstructionScript)