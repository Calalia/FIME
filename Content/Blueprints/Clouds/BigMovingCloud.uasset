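; BigMovingCloud is a large background cloud actor that drifts along its Y axis and recycles itself.
; It picks a random mesh from CloudMeshArray on BeginPlay and moves by Movespeed every tick, without delta-time scaling.
; Past CloudMaxDistance in world Y, it wraps to a fixed far-negative Y with randomized X, height, scale and mesh, reusing one actor as an endless stream of varied clouds.
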(event EventTick
  (params (DeltaSeconds :type Float%20%28single-precision%29))
  (bind _returnvalue (Math|Random|RandomFloatinRange 2e+02 8e+02))
  (bind _defaultsceneroot (Variables|Default|GetDefaultSceneRoot))
  (if (> (.y (Transformation|GetWorldLocation _defaultsceneroot)) (Variables|Default|GetCloudMaxDistance))
    (Transformation|SetWorldTransform _defaultsceneroot (Math|Transform|MakeTransform (Math|Vector|MakeVector (Math|Random|RandomFloatinRange -3e+05 3e+05) -6e+05 (Math|Random|RandomFloatinRange -9e+04 -9.6e+04)) "0, 0, 0" (Math|Vector|MakeVector _returnvalue _returnvalue (/ _returnvalue 1.0))) false false)
    (Components|StaticMesh|SetStaticMesh (Variables|Default|GetSphere) (Utilities|Array|Get(acopy) (Variables|Default|GetCloudMeshArray) (Math|Random|RandomIntegerinRange 0 5)))
    (else
      (Class|SceneComponent|AddLocalTransform _defaultsceneroot (Math|Transform|MakeTransform (Math|Vector|MakeVector 0.0 (Variables|Default|GetMovespeed) 0.0) "0, 0, 0" "3.000000,3.000000,3.000000") false false))))

(event EventBeginPlay
  (Components|StaticMesh|SetStaticMesh (Variables|Default|GetSphere) (Utilities|Array|Get(acopy) (Variables|Default|GetCloudMeshArray) (Math|Random|RandomIntegerinRange 0 4))))

(fn ConstructionScript)