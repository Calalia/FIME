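; Cloud controller actor that populates the sky with moving clouds, spawning a single EdgeCloud at the origin on BeginPlay.
; Each Tick spawns at most one cloud, filling the big, then medium, then small tier up to its maximum count.
; Each tier spawns at random positions within its own area and negative height band, with medium and small clouds also getting random scale.
; Counts come from a GetAllActorsOfClass search run on Tick.
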(event EventBeginPlay
  (Game|SpawnActorfromClass "/Game/Blueprints/Clouds/EdgeCloud.EdgeCloud_C" (Math|Transform|MakeTransform "0, 0, 0") "Undefined" 0 0))

(event EventTick
  (params (DeltaSeconds :type Float%20%28single-precision%29))
  (bind _returnvalue (Math|Random|RandomFloatinRange 1.1 2.8))
  (bind _returnvalue_2 (Math|Random|RandomFloatinRange 0.1 0.3))
  (if (< (Utilities|Array|Length (stale _outactors)) (Variables|Default|GetMaxBigCloudAmount))
    (bind _outactors (Actor|GetAllActorsOfClass "/Game/Blueprints/Clouds/BigMovingCloud.BigMovingCloud_C"))
    (Game|SpawnActorfromClass "/Game/Blueprints/Clouds/BigMovingCloud.BigMovingCloud_C" (Math|Transform|MakeTransform (Math|Vector|MakeVector (Math|Random|RandomFloatinRange -3e+05 3e+05) (Math|Random|RandomFloatinRange -6e+05 6e+05) (Math|Random|RandomFloatinRange -9e+04 -9.6e+04)) "0, 0, 0" "3.000000,3.000000,2.000000") "Undefined" 0 0)
    (elif (< (Utilities|Array|Length (stale _outactors_2)) (Variables|Default|GetMaxMediumCloudAmount))
      (bind _outactors_2 (Actor|GetAllActorsOfClass "/Game/Blueprints/Clouds/MediumMovingCloud.MediumMovingCloud_C"))
      (Game|SpawnActorfromClass "/Game/Blueprints/Clouds/MediumMovingCloud.MediumMovingCloud_C" (Math|Transform|MakeTransform (Math|Vector|MakeVector (Math|Random|RandomFloatinRange -1e+05 1e+05) (Math|Random|RandomFloatinRange -3e+05 3e+05) (Math|Random|RandomFloatinRange -5.5e+04 -7.6e+04)) "0, 0, 0" (Math|Vector|MakeVector _returnvalue _returnvalue (Math|Random|RandomFloatinRange 0.5 1.1))) "Undefined" 0 0)
      (elif (< (Utilities|Array|Length (stale _outactors_3)) (Variables|Default|GetMaxSmallCloudAmount))
        (bind _outactors_3 (Actor|GetAllActorsOfClass "/Game/Blueprints/Clouds/SmallMovingCloud.SmallMovingCloud_C"))
        (Game|SpawnActorfromClass "/Game/Blueprints/Clouds/SmallMovingCloud.SmallMovingCloud_C" (Math|Transform|MakeTransform (Math|Vector|MakeVector (Math|Random|RandomFloatinRange -1e+05 1e+05) (Math|Random|RandomFloatinRange -3e+05 3e+05) (Math|Random|RandomFloatinRange -3e+02 -1e+03)) "0, 0, 0" (Math|Vector|MakeVector _returnvalue_2 _returnvalue_2 (Math|Random|RandomFloatinRange 0.1 0.2))) "Undefined" 0 0)))))

(fn ConstructionScript)