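; MediumMovingCloud is a background cloud actor that drifts along Y and recycles itself to keep clouds moving across the scene.
; BeginPlay gives the Sphere component a random mesh from CloudMeshArray.
; Each Tick moves the root by Movespeed in local Y, unscaled by delta time.
; Past CloudMaxDistance, it jumps to a fixed starting Y with random X, height and scale, and picks a new mesh.
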(event EventTick
  (params (DeltaSeconds :type Float%20%28single-precision%29))
  (bind _returnvalue (Math|Random|RandomFloatinRange 1.1 2.2))
  (bind _defaultsceneroot (Variables|Default|GetDefaultSceneRoot))
  (if (> (.y (Transformation|GetWorldLocation _defaultsceneroot)) (Variables|Default|GetCloudMaxDistance))
    (Transformation|SetWorldTransform _defaultsceneroot (Math|Transform|MakeTransform (Math|Vector|MakeVector (Math|Random|RandomFloatinRange -1e+05 1e+05) -6e+05 (Math|Random|RandomFloatinRange -5.5e+04 -7.6e+04)) "0, 0, 0" (Math|Vector|MakeVector _returnvalue _returnvalue _returnvalue)) false false)
    (Components|StaticMesh|SetStaticMesh (Variables|Default|GetSphere) (Utilities|Array|Get(acopy) (Variables|Default|GetCloudMeshArray) (Math|Random|RandomIntegerinRange 0 4)))
    (else
      (Class|SceneComponent|AddLocalTransform _defaultsceneroot (Math|Transform|MakeTransform (Math|Vector|MakeVector 0.0 (Variables|Default|GetMovespeed) 0.0) "0, 0, 0" "2.000000,2.000000,2.000000") false false))))

(event EventBeginPlay
  (Components|StaticMesh|SetStaticMesh (Variables|Default|GetSphere) (Utilities|Array|Get(acopy) (Variables|Default|GetCloudMeshArray) (Math|Random|RandomIntegerinRange 0 4))))

(fn ConstructionScript)