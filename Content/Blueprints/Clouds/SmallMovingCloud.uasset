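; Small background cloud actor that drifts across the level and recycles itself endlessly.
; BeginPlay gives the Sphere component a random mesh from CloudMeshArray for variety.
; Tick moves the root along local Y by a fixed per-frame Movespeed, without delta-time scaling.
; Once world Y exceeds CloudMaxDistance, it jumps back to a far negative Y with randomized X, height and per-axis scale, keeping the same mesh.
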(event EventTick
  (params (DeltaSeconds :type Float%20%28single-precision%29))
  (bind _returnvalue (Math|Random|RandomFloatinRange 0.1 0.3))
  (bind _defaultsceneroot (Variables|Default|GetDefaultSceneRoot))
  (if (> (.y (Transformation|GetWorldLocation _defaultsceneroot)) (Variables|Default|GetCloudMaxDistance))
    (Transformation|SetWorldTransform _defaultsceneroot (Math|Transform|MakeTransform (Math|Vector|MakeVector (Math|Random|RandomFloatinRange -1e+05 1e+05) -6e+05 (Math|Random|RandomFloatinRange -3e+02 -2.2e+04)) "0, 0, 0" (Math|Vector|MakeVector _returnvalue _returnvalue _returnvalue)) false false)
    (else
      (Class|SceneComponent|AddLocalTransform _defaultsceneroot (Math|Transform|MakeTransform (Math|Vector|MakeVector 0.0 (Variables|Default|GetMovespeed) 0.0) "0, 0, 0" "0.500000,0.500000,0.500000") false false))))

(event EventBeginPlay
  (Components|StaticMesh|SetStaticMesh (Variables|Default|GetSphere) (Utilities|Array|Get(acopy) (Variables|Default|GetCloudMeshArray) (Math|Random|RandomIntegerinRange 0 4))))

(fn ConstructionScript)