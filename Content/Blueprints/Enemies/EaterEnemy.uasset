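; Enemy that moves to a random elevated waypoint around the Castle, then heads for the Castle, diverting to eat buildings along the way.
; Tick steers it straight at its target position until it starts eating.
; A targeting area picks targetable buildings, and collider contact asks the target to start being eaten.
; Refused or untargetable targets trigger a switch to the closest allowed building; untargetable ones can fall back to the waypoint.
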(event OnComponentBeginOverlap(TargetingArea)
  (params (OverlappedComponent :type Primitive%20Component%20Object%20Reference) (OtherActor :type Actor%20Object%20Reference) (OtherComp :type Primitive%20Component%20Object%20Reference) (OtherBodyIndex :type Integer) (bFromSweep :type Boolean) (SweepResult :type Hit%20Result%20Structure%20%28by%20ref%29))
  ;[1 1 1] Targeting and untargeting of buildings Inside TargetingArea
  (bind _asparent_building (Utilities|Casting|CastToParentBuilding OtherActor))
  (if (Default|IsTargetable _asparent_building)
    (Utilities|Array|AddUnique (Variables|Default|GetTargetList) _asparent_building)
    (Game|BindEventtoOnDestroyed _asparent_building (delegate Custom|RemoveDestroyedTarget))
    (EventDispatchers|BindEventtoOnBecomeUntargetable _asparent_building (delegate Custom|SwitchIfNotEating))
    (if (not (Utilities|IsValid (Variables|Default|GetTargetStructure)))
      (bind _output_get (Variables|Default|SetTargetStructure _asparent_building))
      (Variables|Default|SetTargetPosition (Transformation|GetActorLocation _output_get)))))

(event OnComponentEndOverlap(TargetingArea)
  (params (OverlappedComponent :type Primitive%20Component%20Object%20Reference) (OtherActor :type Actor%20Object%20Reference) (OtherComp :type Primitive%20Component%20Object%20Reference) (OtherBodyIndex :type Integer))
  ;[1 1 1] Targeting and untargeting of buildings Inside TargetingArea
  (bind _asparent_building (Utilities|Casting|CastToParentBuilding OtherActor))
  (Utilities|Array|RemoveItem (Variables|Default|GetTargetList) _asparent_building))

(event OnComponentBeginOverlap(Collider)
  (params (OverlappedComponent :type Primitive%20Component%20Object%20Reference) (OtherActor :type Actor%20Object%20Reference) (OtherComp :type Primitive%20Component%20Object%20Reference) (OtherBodyIndex :type Integer) (bFromSweep :type Boolean) (SweepResult :type Hit%20Result%20Structure%20%28by%20ref%29))
  (bind (_found _closesttarget) (CallFunction|GetClosestAllowedTarget))
  ;[1 1 1] Start Eating when collided with a building
  (bind _asparent_building (Utilities|Casting|CastToParentBuilding OtherActor))
  (if (== _asparent_building (Variables|Default|GetTargetStructure))
    (if (Default|IsTargetable _asparent_building)
      (if (not (Variables|Default|GetEating))
        (bind _success (Default|StartEating _asparent_building self))
        (if _success
          (Variables|Default|SetEating true)
          (else
            (if _found :!label _label
              (CallFunction|SetTarget _closesttarget)))))
      (else
        (goto _label)))))

(event Custom|RemoveDestroyedTarget
  (params (DestroyedActor :type Actor%20Object%20Reference))
  ;[1 1 1] Targeting and untargeting of buildings Inside TargetingArea
  (bind _asparent_building (Utilities|Casting|CastToParentBuilding DestroyedActor))
  (Utilities|Array|RemoveItem (Variables|Default|GetTargetList) _asparent_building))

(event Custom|SwitchIfNotEating
  (params (Sender :type Parent%20Building%20Object%20Reference))
  (bind (_found _closesttarget) (CallFunction|GetClosestAllowedTarget))
  (bind _targetstructure (Variables|Default|GetTargetStructure))
  ;[1 1 1] Targeting and untargeting of buildings Inside TargetingArea
  (if (and (Utilities|IsValid _targetstructure) (== Sender _targetstructure))
    (if (not (Default|IsEatingThis (Variables|Default|GetTargetStructure) self))
      (if _found
        (CallFunction|SetTarget _closesttarget)
        (else
          (CallFunction|ContinuetoDestination))))))

(event EventBeginPlay
  (bind _outactors (Actor|GetAllActorsOfClass "/Game/Blueprints/Castle.Castle_C"))
  (if (> (Utilities|Array|Length _outactors) 0)
    (bind _output_get (Variables|Default|SetWayPoint (Math|Vector|MakeVector (+ (Math|Random|RandomFloatinRange -5e+03 5e+03) (.x (Transformation|GetActorLocation (Utilities|Array|Get(acopy) _outactors)))) (+ (Math|Random|RandomFloatinRange -5e+03 5e+03) (.y (Transformation|GetActorLocation (Utilities|Array|Get(acopy) _outactors)))) 2e+03)))
    (Variables|Default|SetTargetPosition _output_get)))

(event EventTick
  (params (DeltaSeconds :type Float%20%28single-precision%29))
  (bind _returnvalue (Transformation|GetActorLocation))
  ;[1 1 1] Event Tick, if not Eating move to target
  (if (not (Variables|Default|GetEating))
    (Transformation|SetActorLocation (+ _returnvalue (* (Math|Vector|Normalize (- (Variables|Default|GetTargetPosition) _returnvalue)) (* DeltaSeconds (Variables|Default|GetEnemySpeed)))) false false)
    (Transformation|SetActorRotation (Math|Rotator|MakeRotfromXZ (Math|Vector|Normalize (- (Variables|Default|GetTargetPosition) _returnvalue)) (Math|Vector|VectorUp)))
    ;;[1 1 1] At Starting destination, set destination to castle location
    (if (and (Math|Vector|Equal(Vector) (Variables|Default|GetWayPoint) (Variables|Default|GetTargetPosition) 0.0001) (Math|Vector|Equal(Vector) (Variables|Default|GetTargetPosition) (Transformation|GetActorLocation) 0.0001))
      (bind _outactors (Actor|GetAllActorsOfClass "/Game/Blueprints/Castle.Castle_C"))
      (if (> (Utilities|Array|Length _outactors) 0)
        (Variables|Default|SetTargetPosition (Transformation|GetActorLocation (Utilities|Array|Get(acopy) _outactors)))))))

(fn ConstructionScript
  (|CallParentFunction))

(fn GetClosestAllowedTarget
  (CallFunction|CheckTargetsinArea)
  (for _array_element (Variables|Default|GetTargetList)
    (if (Default|IsTargetable _array_element)
      (if (or (== (LocalVariables|GetShortestDistance) -1.0) (< (Math|Vector|VectorLength (- (Transformation|GetActorLocation _array_element) (Transformation|GetActorLocation))) (LocalVariables|GetShortestDistance)))
        (LocalVariables|SetShortestDistance (Math|Vector|VectorLength (- (Transformation|GetActorLocation _array_element) (Transformation|GetActorLocation))))
        (LocalVariables|SetTarget _array_element))))
  (return (!= (LocalVariables|GetShortestDistance) -1.0) (LocalVariables|GetTarget)))

(fn CheckTargetsinArea
  ;[1 1 1] Wipes and refills TargetList
  (Utilities|Array|Clear (Variables|Default|GetTargetList))
  (for _array_element (Collision|GetOverlappingActors (Variables|Default|GetTargetingArea) "/Game/Blueprints/ParentBuilding.ParentBuilding_C" :!class /Script/Engine.PrimitiveComponent)
    (bind _asparent_building (Utilities|Casting|CastToParentBuilding _array_element))
    (Utilities|Array|Add (Variables|Default|GetTargetList) _asparent_building)))

(fn SetTarget
  (params (NewTarget :type Parent%20Building%20Object%20Reference))
  (bind _output_get (Variables|Default|SetTargetStructure NewTarget))
  (Variables|Default|SetTargetPosition (Transformation|GetActorLocation _output_get)))

(fn ContinuetoDestination
  (Variables|Default|SetTargetPosition (Variables|Default|GetWayPoint)))