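; ParentEnemy is an enemy Blueprint, apparently a base class, that provides damage, death and targetability logic.
; TakeDamage skips living enemies with Health at the -1 sentinel, otherwise sets Health to Amount minus Health, an inverted subtraction, and flags Dead at zero or below.
; TakeDamage never calls Die, which separately sets Dead and destroys the actor.
; IsTargetable returns true while the enemy is not Dead.
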(fn ConstructionScript)

(fn TakeDamage
  (params (Amount :type Float%20%28single-precision%29))
  (if (not (and (not (Variables|Default|GetDead)) (== (Variables|Default|GetHealth) -1.0)))
    (bind _output_get (Variables|Default|SetHealth (- Amount (Variables|Default|GetHealth))))
    (Variables|Default|SetDead (<= _output_get 0.0))))

(fn Die
  (Variables|Default|SetDead true)
  (Actor|DestroyActor))

(fn IsTargetable
  (return (not (Variables|Default|GetDead))))