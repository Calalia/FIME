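; Player controller for a free strategy-style camera, driving a CameraPawn with the mouse cursor shown.
; Axis inputs move the pawn relative to its facing at a speed scaled by zoom, while zoom changes the clamped spring arm length.
; Holding Pan opens gates that let the mouse rotate yaw and clamped pitch, and suspends movement.
; Otherwise, a ScreenEdgeMovement macro scrolls the camera when the cursor nears the viewport edges.
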(event EventBeginPlay
  (Variables|Default|SetbShowMouseCursor true)
  (bind _ascamera_pawn (Utilities|Casting|CastToCameraPawn (Game|Player|GetPlayerPawn 0)))
  (Variables|References|SetCameraPawnRef _ascamera_pawn))

(event Input|ActionEvents|InputActionPan
  (params (Key :type Key%20Structure))
  (bind _camerapawnref (Variables|References|GetCameraPawnRef))
  (bind _returnvalue (Transformation|GetActorRotation _camerapawnref))
  ;[1 1 1] Pan X
  (:Pressed
    (Variables|Default|SetDisableCamMovement true)
    (Utilities|FlowControl|Gate true) ; enters at Open
  )
  (:Released
    (Variables|Default|SetDisableCamMovement false)
    (Utilities|FlowControl|Gate true) ; enters at Close
  ))

(event Input|ActionEvents|InputActionPan
  (params (Key :type Key%20Structure))
  (bind _camerapawnref (Variables|References|GetCameraPawnRef))
  (bind _returnvalue (Transformation|GetActorRotation _camerapawnref))
  ;[1 1 1] Pan Y
  (:Pressed
    (Variables|Default|SetDisableCamMovement true)
    (Utilities|FlowControl|Gate true) ; enters at Open
  )
  (:Released
    (Variables|Default|SetDisableCamMovement false)
    (Utilities|FlowControl|Gate true) ; enters at Close
  ))

(event Input|AxisEvents|InputAxisHorizontal
  (params (AxisValue :type Float%20%28single-precision%29))
  (bind _camerapawnref (Variables|References|GetCameraPawnRef))
  ;[1 1 1] Movement Horizontal
  (if (not (Variables|Default|GetDisableCamMovement))
    (Transformation|SetActorTransform _camerapawnref (Utilities|MovementHorizontal AxisValue (CallFunction|ZoomMovementSpeed) _camerapawnref))))

(event Input|AxisEvents|InputAxisVertical
  (params (AxisValue :type Float%20%28single-precision%29))
  (bind _camerapawnref (Variables|References|GetCameraPawnRef))
  ;[1 1 1] Movement Vertical
  (if (not (Variables|Default|GetDisableCamMovement))
    (Transformation|SetActorTransform _camerapawnref (Utilities|MovementVertical AxisValue (CallFunction|ZoomMovementSpeed) _camerapawnref))))

(event Input|AxisEvents|InputAxisZoom
  (params (AxisValue :type Float%20%28single-precision%29))
  (bind _camerapawnref (Variables|References|GetCameraPawnRef))
  (bind _springarm (Variables|/Game/Blueprints/CameraPawn.CameraPawn_C|GetSpringArm _camerapawnref))
  ;[1 1 1] Zoom
  (Variables|/Script/Engine.SpringArmComponent|SetTargetArmLength _springarm (Math|Float|Clamp(Float) (+ (Variables|/Script/Engine.SpringArmComponent|GetTargetArmLength _springarm) (* AxisValue (Variables|Default|GetZoomSensitivity))) (Variables|Default|GetMinZoomDistance) (Variables|Default|GetMaxZoomDistance))))

(event Input|MouseEvents|MouseX
  (params (AxisValue :type Float%20%28single-precision%29))
  (bind _camerapawnref (Variables|References|GetCameraPawnRef))
  (bind _returnvalue (Transformation|GetActorRotation _camerapawnref))
  ;[1 1 1] Pan X
  (Utilities|FlowControl|Sequence
    (:then_0
      (Utilities|FlowControl|Gate true
        (:Exit
          (Transformation|SetActorRotation (Variables|References|GetCameraPawnRef) (Math|Rotator|MakeRotator (.roll _returnvalue) (.pitch _returnvalue) (+ (.yaw _returnvalue) (* (Variables|Default|GetPanSensitivity) AxisValue)))))))
    (:then_1
      ;[1 1 1] Screen Edge Movement
      (if (not (Variables|Default|GetDisableCamMovement))
        (bind (_cammovehorizontal _cammovevertical) (Utilities|ScreenEdgeMovement)
          (:Exec
            (Transformation|AddActorLocalOffset (Variables|References|GetCameraPawnRef) (Math|Vector|MakeVector _cammovevertical _cammovehorizontal 0.0) false false)))))))

(event Input|MouseEvents|MouseY
  (params (AxisValue :type Float%20%28single-precision%29))
  (bind _camerapawnref (Variables|References|GetCameraPawnRef))
  (bind _returnvalue (Transformation|GetActorRotation _camerapawnref))
  ;[1 1 1] Pan Y
  (Utilities|FlowControl|Sequence
    (:then_0
      (Utilities|FlowControl|Gate true
        (:Exit
          (Transformation|SetActorRotation (Variables|References|GetCameraPawnRef) (Math|Rotator|MakeRotator (.roll _returnvalue) (Math|Float|Clamp(Float) (+ (.pitch _returnvalue) (* (Variables|Default|GetPanSensitivity) AxisValue)) -15.0 45.0) (.yaw _returnvalue))))))
    (:then_1
      ;[1 1 1] Screen Edge Movement
      (if (not (Variables|Default|GetDisableCamMovement))
        (Utilities|ScreenEdgeMovement) ; enters at MouseY
      ))))

(fn ConstructionScript)

(fn ZoomMovementSpeed
  (return (Math|Float|Clamp(Float) (/ (Variables|/Script/Engine.SpringArmComponent|GetTargetArmLength (Variables|/Game/Blueprints/CameraPawn.CameraPawn_C|GetSpringArm (Variables|References|GetCameraPawnRef))) 1e+02) 5.0 2e+01)))