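; House actor that assembles a randomized building from static mesh components in its Construction Script.
; When ItemToSpawn is not valid, it adds a random base and roof, then spawns doors and windows at transforms taken from placeholder slot components.
; One roll picks both the wooden door position and the main door mesh, with one variant sometimes gaining a shelter.
; Windows fill a random number of slots, removing each used slot to avoid overlaps.
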(fn ConstructionScript
  (CallFunction|SpawnExteriorItems))

(fn SpawnExteriorItems
  (Utilities|IsValid (Variables|Default|GetItemToSpawn)
    (:Is%20Not%20Valid
      (Utilities|FlowControl|Sequence
        (:then_0
          (bind _returnvalue (AddComponent|AddStaticMeshComponent false (Transformation|GetRelativeTransform (Variables|Default|GetBasePosition))))
          (Components|StaticMesh|SetStaticMesh _returnvalue (Utilities|Array|Get(acopy) (Variables|Default|GetHouseBaseArray) (Math|Random|RandomIntegerinRange 0 2))))
        (:then_1
          (CallFunction|SpawnRoof))
        (:then_2
          (CallFunction|SpawnDoor))
        (:then_3
          (CallFunction|SpawnWindow))))))

(fn SpawnRoof
  (bind _returnvalue (AddComponent|AddStaticMeshComponent false (Transformation|GetRelativeTransform (Variables|Default|GetRoofSpawnPos))))
  (Components|StaticMesh|SetStaticMesh _returnvalue (Utilities|Array|Get(acopy) (Variables|Default|GetRoofsToSpawn) (Math|Random|RandomIntegerinRange 0 2))))

(fn SpawnWindow
  (bind _output_get (Variables|Default|SetWindowPosArray (Utilities|Array|MakeArray (Variables|Default|GetSlot2ndWindow1) (Variables|Default|GetSlot2ndWindow2) (Variables|Default|GetSlot2ndWindow3) (Variables|Default|GetSlot2ndWindow4) (Variables|Default|GetSlot2ndWindow5) (Variables|Default|GetSlot2ndWindow6) (Variables|Default|GetSlot2ndWindow7) (Variables|Default|GetSlot2ndWindow8) (Variables|Default|GetSlot1stWindow1) (Variables|Default|GetSlot1stWindow2) (Variables|Default|GetSlot1stWindow3) (Variables|Default|GetSlot1stWindow4) (Variables|Default|GetSlot1stWindow5) (Variables|Default|GetSlot1stWindow6) (Variables|Default|GetSlot1stWindow7))))
  (for _index (range 1 (Math|Random|RandomIntegerinRange 3 8))
    (bind _output_get_2 (LocalVariables|SetWindowToSpawn (Math|Random|RandomIntegerinRange 0 (- (Utilities|Array|Length _output_get) 1))))
    (bind _returnvalue (AddComponent|AddStaticMeshComponent false (Transformation|GetRelativeTransform (Utilities|Array|Get(acopy) _output_get _output_get_2))))
    (Components|StaticMesh|SetStaticMesh _returnvalue (Utilities|Array|Get(acopy) (Variables|Default|GetWindowMeshArray) (Math|Random|RandomIntegerinRange 0 2)))
    (Utilities|Array|RemoveIndex (Variables|Default|GetWindowPosArray) (LocalVariables|GetWindowToSpawn))))

(fn SpawnDoor
  (bind _woodendoorspawnpositions2 (Variables|Default|GetWoodenDoorSpawnPositions2))
  (bind _woodendoorspawnpositions3 (Variables|Default|GetWoodenDoorSpawnPositions3))
  (bind _woodendoorspawnpositions1 (Variables|Default|GetWoodenDoorSpawnPositions1))
  (bind _array (Utilities|Array|MakeArray _woodendoorspawnpositions1 _woodendoorspawnpositions2 _woodendoorspawnpositions3))
  (Variables|Default|SetWoodenDoorSpawnPosArray _array)
  (bind _output_get (Variables|Default|SetDoorInt (Math|Random|RandomIntegerinRange 0 1)))
  (bind _returnvalue (AddComponent|AddStaticMeshComponent false (Transformation|GetRelativeTransform (Utilities|Array|Get(acopy) _array _output_get))))
  (Components|StaticMesh|SetStaticMesh _returnvalue (Variables|Default|GetWoodenDoorRef))
  (bind _returnvalue_2 (AddComponent|AddStaticMeshComponent false (Transformation|GetRelativeTransform (Variables|Default|GetDoorSpawnPos))))
  (Components|StaticMesh|SetStaticMesh _returnvalue_2 (Utilities|Array|Get(acopy) (Variables|Default|GetDoorsToSpawn) _output_get))
  (if (== (Variables|Default|GetDoorInt) 1)
    (if (Math|Random|RandomBool)
      (bind _returnvalue_3 (AddComponent|AddStaticMeshComponent false (Transformation|GetRelativeTransform (Variables|Default|GetDoorShelterPos))))
      (Components|StaticMesh|SetStaticMesh _returnvalue_3 (Utilities|Array|Get(acopy) (Variables|Default|GetDoorsToSpawn) 2)))))