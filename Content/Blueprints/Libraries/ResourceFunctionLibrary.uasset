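; Blueprint function library that does arithmetic on resource amounts of Food, Wood, Stone and Crystal.
; AddResources sums two resource sets field by field and always reports success.
; SubtractResources returns the per-field differences without clamping.
; Its Success output checks that every difference is non-negative, but a constant false in the AND chain makes it always false.
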(fn AddResources
  (params (Param1 :type Resource%20Struct%20Structure) (Param2 :type Resource%20Struct%20Structure))
  (bind (_food _wood _stone _crystal) (Utilities|Struct|BreakResourceStruct Param1))
  (bind (_food_2 _wood_2 _stone_2 _crystal_2) (Utilities|Struct|BreakResourceStruct Param2))
  (return (Utilities|Struct|MakeResourceStruct (+ _food _food_2) (+ _wood _wood_2) (+ _stone _stone_2) (+ _crystal _crystal_2)) true))

(fn SubtractResources
  (params (Param1 :type Resource%20Struct%20Structure) (Param2 :type Resource%20Struct%20Structure))
  (bind (_food _wood _stone _crystal) (Utilities|Struct|BreakResourceStruct Param1))
  (bind (_food_2 _wood_2 _stone_2 _crystal_2) (Utilities|Struct|BreakResourceStruct Param2))
  (bind _returnvalue (- _crystal _crystal_2))
  (bind _returnvalue_2 (- _stone _stone_2))
  (bind _returnvalue_3 (- _food _food_2))
  (bind _returnvalue_4 (- _wood _wood_2))
  (return (Utilities|Struct|MakeResourceStruct _returnvalue_3 _returnvalue_4 _returnvalue_2 _returnvalue) (Math|Boolean|ANDBoolean false (>= _returnvalue_3 0) (>= _returnvalue_4 0) (>= _returnvalue_2 0) (>= _returnvalue 0))))