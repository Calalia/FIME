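; Base building that a single eater can target and consume over time.
; StartEating claims the building, makes it untargetable, fires OnBecomeUntargetable and binds to the eater's OnDestroyed.
; While eaten, Tick drains SustenanceHP by elapsed time; at zero, both eater and building die.
; If the eater is destroyed first, the building becomes targetable again and its HP snaps back to max.
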(event Custom|BindToEaterOnDestroyed
  (params (Eater :type Parent%20Enemy%20Object%20Reference))
  (Game|BindEventtoOnDestroyed Eater (delegate Custom|OnEaterDestroyedDelegate)))

(event Custom|OnEaterDestroyedDelegate
  (params (DestroyedActor :type Actor%20Object%20Reference))
  (CallFunction|EaterDestroyed))

(event EventBeginPlay)

(event Collision|EventActorBeginOverlap
  (params (OtherActor :type Actor%20Object%20Reference)))

(event EventTick
  (params (DeltaSeconds :type Float%20%28single-precision%29))
  (if (Variables|Default|GetEaten)
    (bind _output_get (Variables|Default|SetSustenanceHP (- (Variables|Default|GetSustenanceHP) DeltaSeconds)))
    (if (<= _output_get 0.0)
      (Default|Die (Variables|Default|GetEater))
      (CallFunction|Die))
    (else
      (Variables|Default|SetSustenanceHP (Variables|Default|GetSustenanceHPMax)))))

(fn ConstructionScript)

(fn IsTargetable
  (return (Variables|Default|GetTargetable)))

(fn StartEating
  (params (Eater :type Parent%20Enemy%20Object%20Reference))
  (if (Variables|Default|GetTargetable)
    (Variables|Default|SetEater Eater)
    (Variables|Default|SetTargetable false)
    (Variables|Default|SetEaten true)
    (Default|CallOnBecomeUntargetable self)
    (CallFunction|BindtoEateronDestroyed (Variables|Default|GetEater))
    (return true)
    (else
      (return false))))

(fn IsEatingThis
  (params (Eater :type Parent%20Enemy%20Object%20Reference))
  (return (== Eater (Variables|Default|GetEater))))

(fn EaterDestroyed
  (Variables|Default|SetEaten false)
  (Variables|Default|SetTargetable true))

(fn Die
  (Actor|DestroyActor))