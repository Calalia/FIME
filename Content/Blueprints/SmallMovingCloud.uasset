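; SmallMovingCloud is a drifting cloud actor that recycles itself to give continuous cloud movement.
; On BeginPlay, its Sphere component takes a random mesh from the first five entries of CloudMeshArray.
; Each Tick moves it along local Y by Movespeed, without delta-time scaling.
; Past CloudMaxDistance on world Y, it teleports back to a fixed negative Y with random X, below-origin height and non-uniform scale, keeping its mesh.
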(event EventTick
  (params (DeltaSeconds :type Float%20%28single-precision%29))
  (bind _returnvalue (Math|Random|RandomFloatinRange 0.2 1.0))
  (bind _sphere (Variables|Default|GetSphere))
  (if (> (.y (Transformation|GetWorldLocation _sphere)) (Variables|Default|GetCloudMaxDistance))
    (Transformation|SetWorldTransform _sphere (Math|Transform|MakeTransform (Math|Vector|MakeVector (Math|Random|RandomFloatinRange -1e+05 1e+05) -1e+05 (* _returnvalue -2.2e+04)) "0, 0, 0" (Math|Vector|MakeVector _returnvalue _returnvalue _returnvalue)) false false)
    (else
      (Class|SceneComponent|AddLocalTransform _sphere (Math|Transform|MakeTransform (Math|Vector|MakeVector 0.0 (Variables|Default|GetMovespeed) 0.0) "0, 0, 0" "1,1,1") false false))))

(event EventBeginPlay
  (Components|StaticMesh|SetStaticMesh (Variables|Default|GetSphere) (Utilities|Array|Get(acopy) (Variables|Default|GetCloudMeshArray) (Math|Random|RandomIntegerinRange 0 4))))

(fn ConstructionScript)