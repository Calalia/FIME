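; Spawner Blueprint with a Plane component that grows in exchange for resources; despite its name, it spawns nothing in this graph.
; Its Select event spends one Resource from the FIMEGameInstance, if any remain, and widens the Plane's X and Y scale by one step.
; The Construction Script also calls Select, while BeginPlay sets the Plane to a fixed starting scale, overriding any earlier growth.
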(event EventBeginPlay
  (Transformation|SetRelativeScale3D (Variables|Default|GetPlane) (Math|Vector|MakeVector 1e+01 1e+01 1.0)))

(event EventSelect
  (bind _plane (Variables|Default|GetPlane))
  (bind _relativescale3d (Variables|/Script/Engine.SceneComponent|GetRelativeScale3D _plane))
  (bind _asfimegame_instance (Utilities|Casting|CastToFIMEGameInstance (Game|GetGameInstance)))
  (if (> (Variables|/Game/Blueprints/FIMEGameInstance.FIMEGameInstance_C|GetResources _asfimegame_instance) 0)
    (Variables|/Game/Blueprints/FIMEGameInstance.FIMEGameInstance_C|SetResources _asfimegame_instance (- (Variables|/Game/Blueprints/FIMEGameInstance.FIMEGameInstance_C|GetResources _asfimegame_instance) 1))
    (Transformation|SetRelativeScale3D _plane (Math|Vector|MakeVector (+ (.x _relativescale3d) 1.0) (+ (.y _relativescale3d) 1.0) (.z _relativescale3d)))))

(fn ConstructionScript
  (CallFunction|Select))