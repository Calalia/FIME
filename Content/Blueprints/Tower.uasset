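; Tower actor that automatically kills enemies entering its target area, acting only while it is not eaten.
; Overlap and destroy events maintain a list of enemies, from which Tick takes the first targetable one and keeps it while valid.
; Firing snaps the turret's yaw toward the target, draws a debug line and calls Die directly, then waits on a cooldown timer.
; With no target, the turret spins idly.
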(event OnComponentBeginOverlap(TargetArea)
  (params (OverlappedComponent :type Primitive%20Component%20Object%20Reference) (OtherActor :type Actor%20Object%20Reference) (OtherComp :type Primitive%20Component%20Object%20Reference) (OtherBodyIndex :type Integer) (bFromSweep :type Boolean) (SweepResult :type Hit%20Result%20Structure%20%28by%20ref%29))
  (bind _asparent_enemy (Utilities|Casting|CastToParentEnemy OtherActor))
  (Utilities|Array|AddUnique (Variables|Default|GetTargetList) _asparent_enemy)
  (Game|BindEventtoOnDestroyed (delegate Custom|RemoveDestroyedTarget)))

(event OnComponentEndOverlap(TargetArea)
  (params (OverlappedComponent :type Primitive%20Component%20Object%20Reference) (OtherActor :type Actor%20Object%20Reference) (OtherComp :type Primitive%20Component%20Object%20Reference) (OtherBodyIndex :type Integer))
  (bind _asparent_enemy (Utilities|Casting|CastToParentEnemy OtherActor))
  (Utilities|Array|RemoveItem (Variables|Default|GetTargetList) _asparent_enemy)
  (Game|UnbindEventfromOnDestroyed _asparent_enemy (delegate Custom|RemoveDestroyedTarget)))

(event Custom|RemoveDestroyedTarget
  (params (DestroyedActor :type Actor%20Object%20Reference))
  (bind _asparent_enemy (Utilities|Casting|CastToParentEnemy DestroyedActor))
  (Utilities|Array|RemoveItem (Variables|Default|GetTargetList) _asparent_enemy))

(event EventBeginPlay
  (|CallParentFunction) ; This node is disabled and will not be called.\nDrag off pins to build functionality.
)

(event Collision|EventActorBeginOverlap
  (params (OtherActor :type Actor%20Object%20Reference))
  (|CallParentFunction OtherActor) ; This node is disabled and will not be called.\nDrag off pins to build functionality.
)

(event EventTick
  (params (DeltaSeconds :type Float%20%28single-precision%29))
  (|CallParentFunction DeltaSeconds)
  (if (not (Variables|Default|GetEaten))
    (CallFunction|TryPickTarget)
    (if (Utilities|IsValid (Variables|Default|GetTarget))
      (if (not (Variables|Default|GetAttackOnCooldown))
        (CallFunction|ShootatTarget)
        (Variables|Default|SetAttackOnCooldown true)
        (Utilities|Time|SetTimerbyFunctionName self "ResetCooldown" (Variables|Default|GetAttackCooldown)))
      (else
        (CallFunction|IdleTick DeltaSeconds)))))

(fn ConstructionScript
  (|CallParentFunction))

(fn TryPickTarget
  (if (not (Utilities|IsValid (Variables|Default|GetTarget)))
    (bind _array_element (Utilities|Array|ForEachLoopwithBreak (Variables|Default|GetTargetList) :!label _label)
      (:LoopBody
        (if (Default|IsTargetable _array_element)
          (Variables|Default|SetTarget _array_element)
          (goto _label Break))))))

(fn ShootatTarget
  (bind _turret (Variables|Default|GetTurret))
  (bind _target (Variables|Default|GetTarget))
  (bind _returnvalue (Transformation|GetWorldLocation _turret))
  (bind _returnvalue_2 (Transformation|GetActorLocation _target))
  (bind _returnvalue_3 (- _returnvalue_2 _returnvalue))
  (Transformation|SetWorldRotation _turret (Math|Rotator|MakeRotfromXZ (Math|Vector|MakeVector (.x _returnvalue_3) (.y _returnvalue_3) 0.0) (Math|Vector|VectorUp)) false false)
  (Rendering|Debug|DrawDebugLine _returnvalue _returnvalue_2 "(R=1.000000,G=0.000000,B=0.000000,A=1.000000)" 2.0 3.0)
  (Default|Die (Variables|Default|GetTarget)))

(fn ResetCooldown
  (Variables|Default|SetAttackOnCooldown false))

(fn IdleTick
  (params (DeltaTime :type Float%20%28single-precision%29))
  (bind _turret (Variables|Default|GetTurret))
  (bind _relativerotation (Variables|/Script/Engine.SceneComponent|GetRelativeRotation _turret))
  (if (Utilities|IsValid _turret)
    (Transformation|SetRelativeRotation _turret (Math|Rotator|MakeRotator (.roll _relativerotation) (.pitch _relativerotation) (+ (* DeltaTime (Variables|Default|GetRotation%20Speed)) (.yaw _relativerotation))) false false)))